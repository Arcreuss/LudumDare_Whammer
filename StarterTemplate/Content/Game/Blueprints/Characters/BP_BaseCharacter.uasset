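; First-person base character with a hammer attack, where any damage or contact with rooms, cracked walls or cracked windows is fatal.
; Wall contact is caught by capsule hit events plus a looping overlap-style capsule trace.
; The attack montage's notify sphere-traces from the camera to apply damage, with cooldown shortened by AttackSpeed.
; Death runs once, posting name (defaulting to Unknown) and score to the leaderboard, then opening the scoreboard level.
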(event `OnTakeAnyDamage_Event` :!signature `self.OnTakeAnyDamage`
  (params (DamagedActor :type "Actor Object Reference") (Damage :type "Float (single-precision)") (DamageType :type "DamageType Object Reference") (InstigatedBy :type "Controller Object Reference") (DamageCauser :type "Actor Object Reference"))
  (`self.Die`))

(event `self.ReceiveBeginPlay`
  (`parent.ReceiveBeginPlay`)
  (`KismetSystemLibrary.K2_SetTimerDelegate` (delegate `CheckForCollisionsWithWalls`) 0.1 true)
  (add `self.OnTakeAnyDamage` (delegate `OnTakeAnyDamage_Event`)))

(event `CheckForCollisionsWithWalls`
  (bind _returnvalue (`self.K2_GetActorLocation`))
  (bind _outhit (`KismetSystemLibrary.CapsuleTraceSingle` _returnvalue _returnvalue 34.0 88.0 "TraceTypeQuery1"))
  (bind (_bblockinghit _binitialoverlap _time _distance _location _impactpoint _normal _impactnormal _physmat _hitactor) (`GameplayStatics.BreakHitResult` _outhit))
  (cast `/Game/Game/Blueprints/LevelActor/BP_Room` _hitactor
    (:`then`
      _)
    (:`CastFailed`
      (cast `/Game/Game/Blueprints/GameObjects/BP_CrackedWall` _hitactor
        (:`then`
          _)
        (:`CastFailed`
          (cast `/Game/Game/Blueprints/GameObjects/BP_CrackedWindows` _hitactor)))))
  (`self.Die`))

(event `self.OnJumped`
  ;[1 0.2249 0.8231] Jump and Land Animations
  (if (`self.IsAttackingAnimation`)
    (`|PlayMontage` (`self.FPSArms`) "/Game/Externals/FPS_Arms/Animations/Montages/AS_Arms_Jump_Montage.AS_Arms_Jump_Montage")))

(event `self.OnLanded`
  (params (Hit :type "HitResult Structure (by ref)"))
  ;[1 0.2249 0.8231] Jump and Land Animations
  (if (`self.IsAttackingAnimation`)
    (`|PlayMontage` (`self.FPSArms`) "/Game/Externals/FPS_Arms/Animations/Montages/AS_Arms_Land_Montage.AS_Arms_Land_Montage")))

(event `self.OnAttack`
  (bind _camera (`self.Camera`))
  (bind _returnvalue (`SceneComponent.K2_GetComponentLocation` _camera))
  (set `self.bCanAttack` false)
  (set `self.IsAttackingAnimation` true)
  (`|PlayMontage` (`self.FPSArms`) "/Game/Externals/FPS_Arms/Animations/Montages/AS_Arms_Attack_Montage.AS_Arms_Attack_Montage" 0.8
    (:`then`
      (`KismetSystemLibrary.Delay` (- 1.0 (/ (`self.AttackSpeed`) 100.0)))
      (set `self.bCanAttack` true))
    (:`OnCompleted`
      (set `self.IsAttackingAnimation` false :!label _label))
    (:`OnInterrupted`
      (goto _label))
    (:`OnNotifyBegin`
      (bind _outhit (`KismetSystemLibrary.SphereTraceSingle` _returnvalue (+ _returnvalue (* (`SceneComponent.GetForwardVector` _camera) (`self.AttackRange`))) 50.0 "TraceTypeQuery3"))
      (`GameplayStatics.ApplyDamage` (`.HitActor` (`GameplayStatics.BreakHitResult` _outhit)) (`self.HammerDamages`) null self))))

(event `Die`
  (`/Engine/EditorBlueprintResources/StandardMacros.DoOnce` false ; Randomly, the hit occur 2 times
    (:`Completed`
      ;[1 1 1] Send the player score to scoreboard
      (bind _asbp_base_game_instance (cast `/Game/Game/Blueprints/GameInstances/BP_BaseGameInstance` (`GameplayStatics.GetGameInstance`)))
      (bind (_name _score) (break `ULPlayer` (`/Game/Game/Blueprints/GameInstances/BP_BaseGameInstance.PlayerInfo` _asbp_base_game_instance)))
      ;;[1 1 1] Ensure no name player
      (if (not (`KismetStringLibrary.NotEqual_StrStr` _name))
        (`/Game/Game/Blueprints/GameInstances/BP_BaseGameInstance.UpdateName` _asbp_base_game_instance "Unknown"))
      (`ULLeaderboardSubsystem.PostPlayer` (subsystem `ULLeaderboardSubsystem`) _name _score)
      (`GameplayStatics.OpenLevelBySoftObjectPtr` "/Game/Game/Levels/Menu/LVL_Scoreboard.LVL_Scoreboard"))))

(event `self.CapsuleComponent.OnComponentHit`
  (params (HitComponent :type "PrimitiveComponent Object Reference") (OtherActor :type "Actor Object Reference") (OtherComp :type "PrimitiveComponent Object Reference") (NormalImpulse :type "Vector Structure") (Hit :type "HitResult Structure (by ref)"))
  (cast `/Game/Game/Blueprints/LevelActor/BP_Room` OtherActor
    (:`then`
      _)
    (:`CastFailed`
      (cast `/Game/Game/Blueprints/GameObjects/BP_CrackedWall` OtherActor
        (:`then`
          _)
        (:`CastFailed`
          (cast `/Game/Game/Blueprints/GameObjects/BP_CrackedWindows` OtherActor)))))
  (`self.Die`))

(fn `UserConstructionScript`)