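; BP_Room is a room level actor that spawns a breakable-looking obstacle, animates its box mesh's scale, then destroys itself.
; OnCountChanged randomly spawns a cracked wall (two in three) or cracked window, attached to BaseMesh in one of three RandomIndex slots.
; A timeline then drives the box's X/Y scale until the room is destroyed.
; Count raises Timeline's play rate, but the window branch plays Timeline_0, whose rate is never set.
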(event `self.OnCountChanged`
  (bind _crackedwindows (`self.CrackedWindows`))
  (bind _randomindex (`self.RandomIndex`))
  (bind _crackedwall (`self.CrackedWall`))
  (bind _randomindex_2 (`self.RandomIndex`))
  (switch `int` (`KismetMathLibrary.RandomInteger` 3)
    (:`Default`
      ;[1 1 1] Mur
      (bind _returnvalue (`|SpawnActorFromClass` "/Game/Game/Blueprints/GameObjects/BP_CrackedWall.BP_CrackedWall_C" (`KismetMathLibrary.MakeTransform` (0.0 0.0 0.0) (struct) (1.0 0.3 1.0)) "AlwaysSpawn" "MultiplyWithRoot" null 1 null :!label _label))
      (set `self.CrackedWall` _returnvalue)
      (`self.K2_AttachToComponent` (`self.CrackedWall`) (`self.BaseMesh`) "None" "SnapToTarget" "SnapToTarget" "KeepWorld" true)
      (if (== _randomindex_2 0)
        (`self.K2_AddActorLocalOffset` _crackedwall (400.0 -700.0 -100.0) false false)
        (`self.K2_AddActorLocalRotation` _crackedwall (struct :`Yaw` -90.0) false false)
        (`TimelineComponent.SetPlayRate` (`self.Timeline`) (`KismetMathLibrary.Conv_IntToDouble` (+ (* (`self.Count`) 0.05) 1)) :!label _label_2)
        (bind (_direction _track_scale) (`Timeline|Timeline`)
          (:`Update`
            (`SceneComponent.SetWorldScale3D` (`self.GetBoxMesh`) (`KismetMathLibrary.MakeVector` _track_scale _track_scale 1.0)))
          (:`Finished`
            (`self.K2_DestroyActor`)))
        (elif (== _randomindex_2 1)
          (`self.K2_AddActorLocalOffset` _crackedwall (0.0 -700.0 -100.0) false false)
          (`self.K2_AddActorLocalRotation` _crackedwall (struct :`Yaw` -90.0) false false)
          (goto _label_2)
          (elif (== _randomindex_2 2)
            (`self.K2_AddActorLocalOffset` _crackedwall (-400.0 -700.0 -100.0) false false)
            (`self.K2_AddActorLocalRotation` _crackedwall (struct :`Yaw` -90.0) false false)
            (goto _label_2)))))
    (:`0`
      (goto _label))
    (:`1`
      (goto _label))
    (:`2`
      ;[1 1 1] Fenêtre
      (bind _returnvalue_2 (`|SpawnActorFromClass` "/Game/Game/Blueprints/GameObjects/BP_CrackedWindows.BP_CrackedWindows_C" (`KismetMathLibrary.MakeTransform` (0.0 0.0 0.0) (struct) (1.0 0.3 1.0)) "AlwaysSpawn" "MultiplyWithRoot" null null))
      (bind _output_get (set `self.CrackedWindows` _returnvalue_2))
      (`self.K2_AttachToComponent` _output_get (`self.BaseMesh`) "None" "SnapToTarget" "SnapToTarget" "KeepWorld" true)
      (if (== _randomindex 0)
        (`self.K2_AddActorLocalOffset` _crackedwindows (400.0 -700.0 -50.0) false false)
        (`self.K2_AddActorLocalRotation` _crackedwindows (struct :`Yaw` -90.0) false false)
        (`TimelineComponent.SetPlayRate` (`self.Timeline`) (`KismetMathLibrary.Conv_IntToDouble` (+ (* (`self.Count`) 0.05) 1)) :!label _label_3)
        (bind (_direction_2 _track_scale_2) (`Timeline|Timeline_0`)
          (:`Update`
            (`SceneComponent.SetWorldScale3D` (`self.GetBoxMesh`) (`KismetMathLibrary.MakeVector` _track_scale_2 _track_scale_2 1.0)))
          (:`Finished`
            (`self.K2_DestroyActor`)))
        (elif (== _randomindex 1)
          (`self.K2_AddActorLocalOffset` _crackedwindows (0.0 -700.0 -50.0) false false)
          (`self.K2_AddActorLocalRotation` _crackedwindows (struct :`Yaw` -90.0) false false)
          (goto _label_3)
          (elif (== _randomindex 2)
            (`self.K2_AddActorLocalOffset` _crackedwindows (-400.0 -700.0 -50.0) false false)
            (`self.K2_AddActorLocalRotation` _crackedwindows (struct :`Yaw` -90.0) false false)
            (goto _label_3)))))))

(fn `UserConstructionScript`)