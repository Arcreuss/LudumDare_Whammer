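; BP_InGameSpotlight is a level actor spotlight that switches on with a sound shortly after play begins.
; On BeginPlay it caches the intensities of its spot light and point light, then sets both to zero.
; After a fixed two-second delay it restores both intensities at once and plays a non-spatialized turn-on sound.
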(event `self.ReceiveBeginPlay`
  (set `self.BaseIntensity` (`LightComponentBase.Intensity` (`self.SpotLightComponent`)))
  (set `self.BasePointIntensity` (`LightComponentBase.Intensity` (`self.PointLight`)))
  (`LightComponent.SetIntensity` (`self.SpotLightComponent`) 0.0)
  (`LightComponent.SetIntensity` (`self.PointLight`) 0.0)
  (`KismetSystemLibrary.Delay` 2.0)
  (`LightComponent.SetIntensity` (`self.SpotLightComponent`) (`self.BaseIntensity`))
  (`LightComponent.SetIntensity` (`self.PointLight`) (`self.BasePointIntensity`))
  (`GameplayStatics.PlaySound2D` "/Game/Game/Sounds/Sources/FX/SpotLightTurningOn/SC_SpotLightTurningOn.SC_SpotLightTurningOn" 1.0 1.0 0.0 null null))

(fn `UserConstructionScript`)