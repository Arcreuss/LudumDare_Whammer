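; BP_LightNeon is a level actor for a ceiling neon lamp that swings continuously once play begins.
; The Swing timeline drives the CellingLamp component's relative Y and Z position, scaled up, and its roll, keeping X, pitch and yaw unchanged.
; When the timeline finishes, its direction selects the Play or Reverse event, ping-ponging the motion indefinitely.
; Reverse also prints a leftover debug string.
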(event `self.ReceiveBeginPlay`
  (bind _celling_lamp (`self.Celling_Lamp`))
  (bind _relativelocation_x (`KismetMathLibrary.BreakVector` (`SceneComponent.RelativeLocation` _celling_lamp)))
  (bind (_relativerotation_roll _relativerotation_pitch _relativerotation_yaw) (`KismetMathLibrary.BreakRotator` (`SceneComponent.RelativeRotation` _celling_lamp)))
  (bind (_direction _movey _movez _rotate) (`Timeline|Swing` :!label _label)
    (:`Update`
      (`SceneComponent.K2_SetRelativeLocationAndRotation` _celling_lamp (`KismetMathLibrary.MakeVector` _relativelocation_x (* _movey 2.0) (* _movez 2.0)) (`KismetMathLibrary.MakeRotator` _rotate _relativerotation_pitch _relativerotation_yaw) false false))
    (:`Finished`
      (switch `ETimelineDirection` _direction
        (:`Forward`
          (`self.Reverse`))
        (:`Backward`
          (`self.Play`))))))

(event `Play`
  (goto _label :!via `PlayFromStart`))

(event `Reverse`
  (`KismetSystemLibrary.PrintString` "sdfgxdgfg")
  (goto _label :!via `ReverseFromEnd`))

(fn `UserConstructionScript`)