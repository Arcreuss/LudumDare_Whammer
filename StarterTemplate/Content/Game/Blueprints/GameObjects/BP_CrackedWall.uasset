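; BP_CrackedWall is a breakable wall that shows more crack decals as character damage lowers its Life.
; On BeginPlay it hides decals according to starting Life and binds damage and destroyed handlers.
; Damage counts only when caused by a BP_BaseCharacter, revealing decal groups at set Life values and firing the destroyed event at zero or below.
; Destruction enables Geometry Collection physics, removes collision components, detaches, then destroys the actor after a delay.
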(event `self.ReceiveBeginPlay`
  (`parent.ReceiveBeginPlay`)
  (switch `int` (`self.Life`)
    (:`1`
      _)
    (:`2`
      (`SceneComponent.SetHiddenInGame` (`self.Decal1`) true false :!label _label)
      (`SceneComponent.SetHiddenInGame` (`self.Decal4`) true false)
      (`SceneComponent.SetHiddenInGame` (`self.Decal3`) true false)
      (`SceneComponent.SetHiddenInGame` (`self.Decal2`) true false))
    (:`3`
      (`SceneComponent.SetHiddenInGame` (`self.Decal7`) true false)
      (`SceneComponent.SetHiddenInGame` (`self.Decal5`) true false)
      (goto _label)))
  (add `self.OnTakeAnyDamage` (delegate `OnTakeAnyDamage_Event`))
  (add `self.OnDestroyed` (delegate `OnDestroyed_Event`)))

(event `OnDestroyed_Event` :!signature `self.OnDestroyed`
  (params (DestroyedActor :type "Actor Object Reference"))
  (`PrimitiveComponent.SetSimulatePhysics` (`self.SM_CrackedWall_GeometryCollection`) true)
  (`ActorComponent.K2_DestroyComponent` (`self.PlayerCollision`))
  (`ActorComponent.K2_DestroyComponent` (`self.HitCollision`))
  (`self.K2_DetachFromActor` "KeepWorld" "KeepWorld" "KeepWorld")
  (`KismetSystemLibrary.Delay` 10.0)
  (`self.K2_DestroyActor`))

(event `OnTakeAnyDamage_Event` :!signature `self.OnTakeAnyDamage`
  (params (DamagedActor :type "Actor Object Reference") (Damage :type "Float (single-precision)") (DamageType :type "DamageType Object Reference") (InstigatedBy :type "Controller Object Reference") (DamageCauser :type "Actor Object Reference"))
  (cast `/Game/Game/Blueprints/Characters/BP_BaseCharacter` DamageCauser)
  (bind _output_get (set `self.Life` (- (`self.Life`) Damage)))
  (if (<= _output_get 0)
    (`self.OnDestroyed_Event` DamagedActor)
    (else
      (switch `int` _output_get
        (:`1`
          (`SceneComponent.SetHiddenInGame` (`self.Decal1`) false false)
          (`SceneComponent.SetHiddenInGame` (`self.Decal4`) false false)
          (`SceneComponent.SetHiddenInGame` (`self.Decal3`) false false)
          (`SceneComponent.SetHiddenInGame` (`self.Decal2`) false false))
        (:`2`
          (`SceneComponent.SetHiddenInGame` (`self.Decal7`) false false)
          (`SceneComponent.SetHiddenInGame` (`self.Decal5`) false false))))))

(fn `UserConstructionScript`)