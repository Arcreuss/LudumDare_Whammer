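; Breakable window actor that shatters when a BP_BaseCharacter is the damage causer, regardless of damage amount.
; BeginPlay binds the damage and destroyed delegates, and a qualifying hit calls the destroyed handler directly.
; That handler enables physics on the window's Geometry Collection, removes the hit and player collision components, detaches the pieces in world space, then destroys the actor after a delay.
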(event `self.ReceiveBeginPlay`
  (`parent.ReceiveBeginPlay`)
  (add `self.OnTakeAnyDamage` (delegate `OnTakeAnyDamage_Event`))
  (add `self.OnDestroyed` (delegate `OnDestroyed_Event`)))

(event `OnDestroyed_Event` :!signature `self.OnDestroyed`
  (params (DestroyedActor :type "Actor Object Reference"))
  (`PrimitiveComponent.SetSimulatePhysics` (`self.SM_Windows_GeometryCollection`) true)
  (`ActorComponent.K2_DestroyComponent` (`self.HitCollision`))
  (`ActorComponent.K2_DestroyComponent` (`self.PlayerCollision`))
  (`SceneComponent.K2_DetachFromComponent` (`self.SM_Windows_GeometryCollection`) "KeepWorld" "KeepWorld" "KeepWorld" true)
  (`KismetSystemLibrary.Delay` 10.0)
  (`self.K2_DestroyActor`))

(event `OnTakeAnyDamage_Event` :!signature `self.OnTakeAnyDamage`
  (params (DamagedActor :type "Actor Object Reference") (Damage :type "Float (single-precision)") (DamageType :type "DamageType Object Reference") (InstigatedBy :type "Controller Object Reference") (DamageCauser :type "Actor Object Reference"))
  (cast `/Game/Game/Blueprints/Characters/BP_BaseCharacter` DamageCauser)
  (`self.OnDestroyed_Event` DamagedActor))

(fn `UserConstructionScript`)