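; BP_BonusMoveSpeed is a damageable bonus pickup that permanently raises the movement speed of the character that destroys it.
; On damage from a BP_BaseCharacter, it stores that character as Player and calls DecreaseLife, whose logic is not defined in this graph.
; When the OnDestroy event fires, it adds a flat amount to the stored Player's MaxWalkSpeed and destroys itself.
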(event `self.ReceiveBeginPlay`
  (add `self.OnTakeAnyDamage` (delegate `OnTakeAnyDamage_Event`))
  (add `self.OnDestroy` (delegate `OnDestroy_Event`)))

(event `OnTakeAnyDamage_Event` :!signature `self.OnTakeAnyDamage`
  (params (DamagedActor :type "Actor Object Reference") (Damage :type "Float (single-precision)") (DamageType :type "DamageType Object Reference") (InstigatedBy :type "Controller Object Reference") (DamageCauser :type "Actor Object Reference"))
  (bind _asbp_base_character (cast `/Game/Game/Blueprints/Characters/BP_BaseCharacter` DamageCauser))
  (set `self.Player` _asbp_base_character)
  (`self.DecreaseLife`))

(event `OnDestroy_Event`
  (bind _charactermovement (`Character.CharacterMovement` (`self.Player`)))
  (set `CharacterMovementComponent.MaxWalkSpeed` (+ (`CharacterMovementComponent.MaxWalkSpeed` _charactermovement) 100.0) _charactermovement)
  (`self.K2_DestroyActor`))

(fn `UserConstructionScript`)