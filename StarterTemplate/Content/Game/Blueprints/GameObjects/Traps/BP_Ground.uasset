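; BP_Ground is a timed floor trap that kills any BP_BaseCharacter overlapping one of its five boxes.
; A timer triggers an earthquake sound and a timeline that moves the floor vertically; after a pause, a second timeline reverses it and rearms with a random delay.
; It coordinates with the saw trap through BP_BaseGameInstance flags, postponing while the saw is on and blocking saw starts during its cycle.
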(event `self.ReceiveBeginPlay`
  (`KismetSystemLibrary.K2_SetTimerDelegate` (delegate `ActivateTrap`) (`self.DelayBeforeActivation`) :!label _label))

(event `ActivateTrap`
  (bind _asbp_base_game_instance (cast `/Game/Game/Blueprints/GameInstances/BP_BaseGameInstance` (`GameplayStatics.GetGameInstance`)))
  (if (`/Game/Game/Blueprints/GameInstances/BP_BaseGameInstance.SawOn` _asbp_base_game_instance)
    (goto _label)
    (else
      (set `/Game/Game/Blueprints/GameInstances/BP_BaseGameInstance.SawCanStart` false _asbp_base_game_instance)
      (`GameplayStatics.PlaySound2D` "/Game/Game/Sounds/Sources/FX/Hearthquake/HearthQuake_Cue.HearthQuake_Cue" 1.0 1.0 0.0 null null)
      (bind (_direction _z) (`Timeline|Activate` :!via `PlayFromStart`)
        (:`Update`
          (`SceneComponent.K2_SetWorldLocation` (`self.Floor`) (`KismetMathLibrary.MakeVector` 0.0 0.0 _z) false false))
        (:`Finished`
          (`KismetSystemLibrary.Delay` 10.0)
          (bind (_direction_2 _z_2) (`Timeline|Timeline` :!via `ReverseFromEnd`)
            (:`Update`
              (`SceneComponent.K2_SetWorldLocation` (`self.Floor`) (`KismetMathLibrary.MakeVector` 0.0 0.0 _z_2) false false))
            (:`Finished`
              (set `/Game/Game/Blueprints/GameInstances/BP_BaseGameInstance.SawCanStart` true _asbp_base_game_instance)
              (set `self.DelayBeforeActivation` (`KismetMathLibrary.RandomFloatInRange` 10.0 30.0))
              (goto _label))))))))

(event `self.Box.OnComponentBeginOverlap`
  (params (OverlappedComponent :type "PrimitiveComponent Object Reference") (OtherActor :type "Actor Object Reference") (OtherComp :type "PrimitiveComponent Object Reference") (OtherBodyIndex :type Integer) (bFromSweep :type Boolean) (SweepResult :type "HitResult Structure (by ref)"))
  (`self.KillPlayer` OtherActor))

(event `self.Box1.OnComponentBeginOverlap`
  (params (OverlappedComponent :type "PrimitiveComponent Object Reference") (OtherActor :type "Actor Object Reference") (OtherComp :type "PrimitiveComponent Object Reference") (OtherBodyIndex :type Integer) (bFromSweep :type Boolean) (SweepResult :type "HitResult Structure (by ref)"))
  (`self.KillPlayer` OtherActor))

(event `self.Box2.OnComponentBeginOverlap`
  (params (OverlappedComponent :type "PrimitiveComponent Object Reference") (OtherActor :type "Actor Object Reference") (OtherComp :type "PrimitiveComponent Object Reference") (OtherBodyIndex :type Integer) (bFromSweep :type Boolean) (SweepResult :type "HitResult Structure (by ref)"))
  (`self.KillPlayer` OtherActor))

(event `self.Box3.OnComponentBeginOverlap`
  (params (OverlappedComponent :type "PrimitiveComponent Object Reference") (OtherActor :type "Actor Object Reference") (OtherComp :type "PrimitiveComponent Object Reference") (OtherBodyIndex :type Integer) (bFromSweep :type Boolean) (SweepResult :type "HitResult Structure (by ref)"))
  (`self.KillPlayer` OtherActor))

(event `self.Box4.OnComponentBeginOverlap`
  (params (OverlappedComponent :type "PrimitiveComponent Object Reference") (OtherActor :type "Actor Object Reference") (OtherComp :type "PrimitiveComponent Object Reference") (OtherBodyIndex :type Integer) (bFromSweep :type Boolean) (SweepResult :type "HitResult Structure (by ref)"))
  (`self.KillPlayer` OtherActor))

(fn `KillPlayer`
  (params (Object :type "Object Object Reference"))
  (bind _asbp_base_character (cast `/Game/Game/Blueprints/Characters/BP_BaseCharacter` Object))
  (`/Game/Game/Blueprints/Characters/BP_BaseCharacter.Die` _asbp_base_character "NewEnumerator0"))

(fn `UserConstructionScript`)