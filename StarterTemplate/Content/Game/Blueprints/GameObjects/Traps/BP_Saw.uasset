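; Saw trap that spins continuously and applies damage when a BP_BaseCharacter overlaps its box while active.
; Chained MoveComponentTo calls rotate the child actor component in two half turns, timed inversely to Speed, and a Reset event restarts the loop.
; SetActive toggles only the damage check, so the rotation keeps running when the trap is inactive.
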(event `self.ReceiveBeginPlay`
  (`KismetSystemLibrary.MoveComponentTo` (`self.ChildActor`) (0.0 0.0 0.0) (struct :`Yaw` 180.0) false false (/ 10.0 (`self.speed`)) :!label _label)
  (`KismetSystemLibrary.MoveComponentTo` (`self.ChildActor`) (0.0 0.0 0.0) (struct :`Yaw` 360.0) false false (/ 10.0 (`self.speed`)))
  (`self.Reset`))

(event `Reset`
  (goto _label))

(event `self.Box.OnComponentBeginOverlap`
  (params (OverlappedComponent :type "PrimitiveComponent Object Reference") (OtherActor :type "Actor Object Reference") (OtherComp :type "PrimitiveComponent Object Reference") (OtherBodyIndex :type Integer) (bFromSweep :type Boolean) (SweepResult :type "HitResult Structure (by ref)"))
  (if (and (`GameplayStatics.ObjectIsA` OtherActor "/Game/Game/Blueprints/Characters/BP_BaseCharacter.BP_BaseCharacter_C") (`self.Active`))
    (`GameplayStatics.ApplyDamage` null 1.0 null self)))

(event `SetActive`
  (params (bActive :type Boolean))
  (set `self.Active` bActive))

(fn `UserConstructionScript`)